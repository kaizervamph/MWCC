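; BP_ClientCounter counts the pedestrian clients standing inside a box area around the actor.
; The ClientCountUpdate event runs a multi box trace for one object type at the actor's location, with no caller in this graph.
; GetPedestriansFromHit collects hit actors that cast to BP_PedestrianBase, and the array length becomes CurrentClients.
; The construction script sizes the Box component with InBoxExtent, the same extent the trace uses.
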(event Custom|ClientCountUpdate
  (bind _returnvalue (Transformation|GetActorLocation))
  (bind _outhits (Class|KismetSystemLibrary|BoxTraceMultiforObjects _returnvalue _returnvalue (Variables|Default|GetIn%20Box%20Extent) "0, 0, 0" (Utilities|Array|MakeArray "ObjectTypeQuery11") false 0 "None" true))
  (bind _pedestrians (CallFunction|GetPedestriansfromHit _outhits))
  (Variables|Default|SetCurrentClients (Utilities|Array|Length _pedestrians)))

(event EventBeginPlay)

(fn ConstructionScript
  (Components|Box|SetBoxExtent (Variables|Default|GetBox) (Variables|Default|GetIn%20Box%20Extent) true))

(fn GetPedestriansfromHit
  (params (Hits :type Array%20of%20Hit%20Result%20Structures))
  (for _array_element Hits
    (bind _asbp_pedestrian_base (Utilities|Casting|CastToBP_PedestrianBase (.HitActor (Collision|BreakHitResult _array_element))))
    (Utilities|Array|Add (LocalVariables|GetTemp) _asbp_pedestrian_base))
  (return (LocalVariables|GetTemp)))