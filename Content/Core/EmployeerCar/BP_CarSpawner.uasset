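; BP_CarSpawner is an actor meant to serve as either a car spawn point or a car remover, selected by IsRemover.
; Spawners start a looping timer with a randomized interval, and non-employee ones count existing actors against a cap.
; The logic is unfinished: actor spawning and destruction nodes are disconnected, so the timer and Box overlap currently neither spawn nor remove anything.
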(event OnComponentBeginOverlap(Box)
  (params (OverlappedComponent :type Primitive%20Component%20Object%20Reference) (OtherActor :type Actor%20Object%20Reference) (OtherComp :type Primitive%20Component%20Object%20Reference) (OtherBodyIndex :type Integer) (bFromSweep :type Boolean) (SweepResult :type Hit%20Result%20Structure%20%28by%20ref%29))
  (if (Variables|Default|GetIsRemover)
    _))

(event Custom|SpawnCars
  (if (not (Variables|Default|GetForEmployees?))
    (bind _outactors (Actor|GetAllActorsOfClass 0))
    (if (>= (Utilities|Array|Length _outactors) 5)
      _)))

(event EventBeginPlay
  (if (not (Variables|Default|GetIsRemover))
    (Utilities|Time|SetTimerbyEvent (delegate Custom|SpawnCars) (Math|Random|RandomFloatinRange (Variables|Default|GetSpawnTimeMin) (Variables|Default|GetSpawnTimeMax)) true)))

(fn ConstructionScript)