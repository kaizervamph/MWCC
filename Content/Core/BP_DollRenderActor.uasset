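; Doll actor that renders procedural character portraits and, in the CharacterCreator level, sets up a body mesh and creator widget with morph targets.
; For batch generation, a looping timer builds cloth and hair meshes, then a SceneCapture2D showing only this actor captures texture and bytes.
; Each render goes to the generator actor in the character struct.
; A DoOnce holds the queue until ResetCapture drops the first entry and reopens it.
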(event Custom|CharacterCreatorLogic
  (bind _returnvalue (UserInterface|CreateWidget 0))
  (Variables|Default|SetCC_Ref _returnvalue)
  (UserInterface|Viewport|AddtoViewport _returnvalue 0)
  (CallFunction|SetBodyMesh (Utilities|Struct|MakeProceduralCharacterStruct 0 0 0 "" "/Game/Assets/Female/SK_Female_01.SK_Female_01" "/Game/Assets/Female/ABP_Female_01.ABP_Female_01_C") (Variables|Default|GetBodyMesh))
  (bind _cc_ref (Variables|Default|GetCC_Ref)
    (:then
      (CallFunction|LoadMorphoTarget _cc_ref (Class|SkeletalMesh|GetAllMorphTargetNames (Variables|/Script/Engine.SkinnedMeshComponent|GetSkeletalMesh (Variables|Default|GetBodyMesh)))))
    (:else)))

(event Custom|GenerateRendersFromAttributes
  (params (Attributes :type Array%20of%20Procedural%20Character%20Struct%20Structures))
  (Variables|Default|SetCharactersToGenerate Attributes)
  (Variables|Default|SetRendersAmount 0)
  (Utilities|FlowControl|Sequence
    (:then_0
      (Utilities|Time|SetTimerbyEvent (delegate Custom|Renders) 0.1 true))))

(event Custom|Renders
  (bind _characterstogenerate (Variables|Default|GetCharactersToGenerate))
  (bind _output (Utilities|Array|Get(acopy) _characterstogenerate))
  (bind _generatoractor (CallFunction|GetGeneratorActor))
  (if (!= (Variables|Default|GetAmount _generatoractor) (Variables|Default|GetRendersAmount))
    (Utilities|FlowControl|DoOnce false
      (:Completed
        (CallFunction|AddClothMeshes (.Cloths (Utilities|Struct|BreakProceduralCharacterStruct _output)) _output)
        (Utilities|FlowControl|Delay 0.1)
        (bind (_sizex _sizey _bytes _texture) (CallFunction|CaptureRender))
        (bind _generatoractor_2 (CallFunction|GetGeneratorActor))
        (bind _structout (Utilities|Struct|SetmembersinProceduralCharacterStruct _output _texture _bytes (Utilities|Struct|MakeInt32Range (Utilities|Struct|MakeInt32RangeBound "Exclusive" _sizex) (Utilities|Struct|MakeInt32RangeBound "Exclusive" _sizey))))
        (CallFunction|AddGeneratedCharacter _generatoractor_2 _structout self)
        (Math|Integer|IncrementInt (Variables|Default|GetRendersAmount))))
    (else
      (Utilities|Time|ClearTimerbyFunctionName self "Renders"))))

(event Custom|ResetCapture
  (bind _characterstogenerate (Variables|Default|GetCharactersToGenerate))
  (bind _output (Utilities|Array|Get(acopy) _characterstogenerate))
  (Utilities|Array|RemoveIndex (Variables|Default|GetCharactersToGenerate))
  (Utilities|FlowControl|DoOnce false) ; enters at Reset
)

(event EventBeginPlay
  (Utilities|Array|Add (Variables|/Script/Engine.SceneCaptureComponent|GetShowOnlyActors (Variables|Default|GetSceneCaptureComponent2D)) self)
  (bind _returnvalue (Game|GetCurrentLevelName true))
  (if (Utilities|Enum|Equal(Enum) _returnvalue "CharacterCreator")
    (CallFunction|CharacterCreatorLogic)))

(fn ConstructionScript)

(fn CaptureRender
  (bind _scenecapturecomponent2d (Variables|Default|GetSceneCaptureComponent2D))
  (bind _texturetarget (Variables|/Script/Engine.SceneCaptureComponent2D|GetTextureTarget _scenecapturecomponent2d))
  (bind _sizex (Variables|/Script/Engine.TextureRenderTarget2D|GetSizeX _texturetarget))
  (bind _sizey (Variables|/Script/Engine.TextureRenderTarget2D|GetSizeY _texturetarget))
  (Rendering|SceneCapture|CaptureScene _scenecapturecomponent2d :!class /Script/Engine.SceneCaptureComponent2D)
  (bind _outimagedata (CallFunction|CaptureSceneTexture (Variables|Default|GetSceneCaptureComponent2D)))
  (bind _returnvalue (CallFunction|CreateTexturefromImageData _outimagedata _sizex _sizey "PF_B8G8R8A8"))
  (return _sizex _sizey _outimagedata _returnvalue))

(fn GetGeneratorActor
  (bind _outactors (Actor|GetAllActorsOfClass 0))
  (return (Utilities|Array|Get(acopy) _outactors)))

(fn AddClothMeshes
  (params (Cloths :type Array%20of%20Cloth%20Struct%20Structures) (CharacterInfo :type Procedural%20Character%20Struct%20Structure%20%28by%20ref%29))
  (bind _meshestemp (LocalVariables|GetMeshesTemp))
  (for _array_element Cloths
    (bind _returnvalue (AddComponent|AddSkeletalMeshComponent false))
    (Utilities|Array|Add (Variables|/Script/Engine.ActorComponent|GetComponentTags _returnvalue) (Utilities|String|StringToName (Utilities|String|EnumtoString (.Type (Utilities|Struct|BreakClothStruct _array_element)))))
    (Utilities|Array|Add (LocalVariables|GetClothsTemp) _returnvalue)
    (Utilities|Array|Add (LocalVariables|GetMeshesTemp) _returnvalue))
  (bind _returnvalue_2 (AddComponent|AddSkeletalMeshComponent false))
  (Utilities|Array|Add (Variables|/Script/Engine.ActorComponent|GetComponentTags _returnvalue_2) "Hair")
  (Utilities|Array|Add _meshestemp _returnvalue_2)
  (CallFunction|ConfigCharacterMeshes self (Variables|Default|GetBodyMesh) _meshestemp CharacterInfo (LocalVariables|GetClothsTemp) _returnvalue_2 Cloths))