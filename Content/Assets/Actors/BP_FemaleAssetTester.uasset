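; Test actor for previewing female character assets: body, hair, cloth and shoes meshes, skin color, morph targets and a looping animation.
; The construction script sets meshes, slaves the other parts to Body's pose, tints skin through dynamic materials, then applies morphs and animation.
; A MorphoTargets map drives weights on all four meshes, with a helper to rebuild it from Body's morph names.
; BeginPlay reapplies morphs and animation; FakeStatistics is an empty stub.
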(event EventBeginPlay
  (CallFunction|ApplyMorphoTargets)
  (CallFunction|ChangeAnimation)
  (CallFunction|FakeStatistics))

(fn ConstructionScript
  (Utilities|FlowControl|Sequence
    (:then_0
      (Class|SkinnedMeshComponent|SetSkeletalMesh (Variables|Default|GetBody) (Variables|Default|GetBodyMesh) true)
      (Class|SkinnedMeshComponent|SetSkeletalMesh (Variables|Default|GetHair) (Variables|Default|GetHairMesh) true)
      (Class|SkinnedMeshComponent|SetSkeletalMesh (Variables|Default|GetCloth) (Variables|Default|GetClothMesh) true)
      (Class|SkinnedMeshComponent|SetMasterPoseComponent (Variables|Default|GetHair) (Variables|Default|GetBody) false))
    (:then_1
      (CallFunction|ChangeSkinColor (Variables|Default|GetSkinColor)))
    (:then_2
      (CallFunction|ApplyMorphoTargets))
    (:then_3
      (CallFunction|ChangeAnimation))))

(fn ChangeSkinColor
  (params (NewColor :type Linear%20Color%20Structure))
  (bind _body (Variables|Default|GetBody))
  (for (_array_element _array_index) (Rendering|Material|GetMaterials _body)
    (bind _returnvalue (Rendering|Material|CreateDynamicMaterialInstance _array_element "None" "None" :!class /Script/Engine.KismetMaterialLibrary))
    (Rendering|Material|SetVectorParameterValue _returnvalue "SkinColor" NewColor :!class /Script/Engine.MaterialInstanceDynamic)
    (Rendering|Material|SetMaterial _body _array_index _returnvalue))
  (return true))

(fn ConfigMorphoTargetsVariable
  (Utilities|Map|Clear (Variables|Default|GetMorphoTargets))
  (for _array_element (Class|SkeletalMesh|GetAllMorphTargetNames (Variables|/Script/Engine.SkinnedMeshComponent|GetSkeletalMesh (Variables|Default|GetBody)))
    (Utilities|Map|Add (Variables|Default|GetMorphoTargets) _array_element 0.0)))

(fn ApplyMorphoTargets
  (bind _morphotargets (Variables|Default|GetMorphoTargets))
  (bind _keys (Utilities|Map|Keys _morphotargets))
  (for _array_element _keys
    (Components|SkeletalMesh|SetMorphTarget (Variables|Default|GetBody) (Utilities|String|StringToName _array_element) (.Value (Utilities|Map|Find _morphotargets _array_element)) true)))

(fn ChangeAnimation
  (bind _body (Variables|Default|GetBody))
  (bind _animation (Variables|Default|GetAnimation))
  (Components|Animation|SetAnimation _body _animation)
  (Components|Animation|PlayAnimation _body _animation true))

(fn FakeStatistics)