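; Animated reflector structure that sweeps at random and flashes between red, green and blue.
; After a random start delay, a looping timer picks a color and applies it to a newly created dynamic material and the child B_Spot_Light's lights.
; Tick eases the reflector mesh's roll toward a random target, while a Delay on Tick periodically re-rolls that target and the RotatingMovement yaw rate.
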(event Custom|ChangeColorLight
  (bind _sm_reflectores (Variables|Default|GetSM_Reflectores))
  (bind _returnvalue (Rendering|Material|CreateDynamicMaterialInstance _sm_reflectores 1 (Rendering|Material|GetMaterial _sm_reflectores 1) "None" :!class /Script/Engine.PrimitiveComponent))
  (Variables|Default|SetColorRand (.OutItem (Utilities|Array|Random (Utilities|Array|MakeArray "(R=0.376036,G=1.000000,B=0.011514,A=1.000000)" "(R=0.144509,G=0.000000,B=1.000000,A=1.000000)" "(R=1.000000,G=0.000000,B=0.000000,A=1.000000)"))))
  (Rendering|Material|SetVectorParameterValue _returnvalue "Color" (Variables|Default|GetColorRand) :!class /Script/Engine.MaterialInstanceDynamic)
  (Rendering|Material|SetMaterial (Variables|Default|GetSM_Reflectores) 1 _returnvalue)
  (bind _asb_spot_light (Utilities|Casting|CastToB_Spot_Light (Variables|/Script/Engine.ChildActorComponent|GetChildActor (Variables|Default|GetB_Spot_Light))))
  (Variables|/Game/InteractiveLights/Blueprints/BaseElements/Light_Base.Light_Base_C|SetLight%20Color _asb_spot_light (Variables|Default|GetColorRand))
  (Rendering|Components|Light|SetLightColor (Variables|/Game/InteractiveLights/Blueprints/BaseElements/Light_Base.Light_Base_C|GetLight _asb_spot_light) (Variables|Default|GetColorRand) true)
  (Rendering|Components|Light|SetLightColor (Variables|/Game/InteractiveLights/Blueprints/B_Spot_Light.B_Spot_Light_C|GetSpotLight _asb_spot_light) (Variables|Default|GetColorRand) true))

(event EventBeginPlay
  (Utilities|FlowControl|Delay (Math|Random|RandomFloatinRange 1.0 5.0))
  (Utilities|Time|SetTimerbyEvent (delegate Custom|ChangeColorLight) 0.5 true))

(event EventTick
  (params (DeltaSeconds :type Float%20%28single-precision%29))
  (bind _sm_reflectores (Variables|Default|GetSM_Reflectores))
  (bind _relativerotation (Variables|/Script/Engine.SceneComponent|GetRelativeRotation _sm_reflectores))
  (bind (_roll _pitch _yaw) (Math|Rotator|BreakRotator _relativerotation))
  (Utilities|FlowControl|Sequence
    (:then_0
      (Transformation|SetRelativeRotation _sm_reflectores (Math|Rotator|MakeRotator (Math|Interpolation|FInterpTo _roll (Variables|Default|GetRandomRot) DeltaSeconds 1.0) _pitch _yaw) false false))
    (:then_1
      (Utilities|FlowControl|Delay 1.0)
      (Variables|Default|SetRandomRot (Math|Random|RandomFloatinRange -9e+01 9e+01))
      (Variables|/Script/Engine.RotatingMovementComponent|SetRotationRate (Variables|Default|GetRotatingMovement) (Math|Rotator|MakeRotator 0.0 0.0 (Math|Random|RandomFloatinRange -1.8e+02 1.8e+02))))))

(fn ConstructionScript)