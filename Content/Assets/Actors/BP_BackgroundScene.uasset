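; Background scene actor with wall and floor mesh groups whose materials are set through the WallMaterial and FloorMaterial variables.
; The construction script runs ChangeWallMaterial, then ChangeFloorMaterial, over the direct static mesh children of SceneWall and SceneFloor.
; Walls get the material on every slot, while floors get it only on the first slot.
; It has no active runtime logic, as the event graph holds only disabled placeholder events.
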(event EventBeginPlay)

(event Collision|EventActorBeginOverlap
  (params (OtherActor :type Actor%20Object%20Reference)))

(event EventTick
  (params (DeltaSeconds :type Float%20%28single-precision%29)))

(fn ConstructionScript
  (Utilities|FlowControl|Sequence
    (:then_0
      (CallFunction|ChangeWallMaterial))
    (:then_1
      (CallFunction|ChangeFloorMaterial))))

(fn ChangeWallMaterial
  (for _array_element (Components|GetChildrenComponents (Variables|Default|GetScene_Wall) false)
    (bind _ascomponente_de_malla_estática (Utilities|Casting|CastToStaticMeshComponent _array_element))
    (for (_ _array_index) (Rendering|Material|GetMaterials _ascomponente_de_malla_estática)
      (Rendering|Material|SetMaterial _ascomponente_de_malla_estática _array_index (Variables|Default|GetWallMaterial))))
  (return true))

(fn ChangeFloorMaterial
  (for _array_element (Components|GetChildrenComponents (Variables|Default|GetScene_Floor) false)
    (bind _ascomponente_de_malla_estática (Utilities|Casting|CastToStaticMeshComponent _array_element))
    (Rendering|Material|SetMaterial _ascomponente_de_malla_estática 0 (Variables|Default|GetFloorMaterial)))
  (return true))