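; BP_LightReflector is a decorative stage-style reflector light that randomly changes color every second.
; On BeginPlay it creates a dynamic material from the skeletal mesh's third material slot and starts a looping timer.
; Each tick of the timer picks red, green or blue and applies it to both that material and the SpotLight.
; It also randomizes a Target angle, which nothing in this graph reads.
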(event Custom|UpdateLights
  (bind _dynmat (Variables|Default|GetDynMat)
    (:then
      (Variables|Default|SetColor (.OutItem (Utilities|Array|Random (Utilities|Array|MakeArray "(R=1.000000,G=0.000000,B=0.000000,A=1.000000)" "(R=0.000000,G=1.000000,B=0.000000,A=1.000000)" "(R=0.000000,G=0.000000,B=1.000000,A=1.000000)"))))
      (Rendering|Material|SetVectorParameterValue _dynmat "Color" (Variables|Default|GetColor) :!class /Script/Engine.MaterialInstanceDynamic)
      (Rendering|Material|SetMaterial (Variables|Default|GetSkeletalMesh) 2 _dynmat)
      (Rendering|Components|Light|SetLightColor (Variables|Default|GetSpotLight) (Variables|Default|GetColor) true)
      (Variables|Default|SetTarget (Math|Random|RandomFloatinRange 0.0 9e+01)))
    (:else)))

(event EventBeginPlay
  (Utilities|Time|SetTimerbyEvent (delegate Custom|UpdateLights) 1.0 true)
  (bind _returnvalue (Rendering|Material|CreateDynamicMaterialInstance (Utilities|Array|Get(acopy) (Rendering|Material|GetMaterials (Variables|Default|GetSkeletalMesh)) 2) "None" "Transient" :!class /Script/Engine.KismetMaterialLibrary))
  (Variables|Default|SetDynMat _returnvalue))

(fn ConstructionScript)