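; BP_LightStation is a decorative light station whose six child-actor BP_LightReflector spotlights blink in two alternating groups.
; On BeginPlay it gathers the spotlights, splits them into two halves and starts a looping one-second timer.
; Each tick of that timer uses a FlipFlop to show one half and hide the other.
; Construction Script logic for pushing intensity and volumetric scattering to the reflectors is disconnected.
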(event Custom|ChangeLights
  (bind _isa (Utilities|FlowControl|FlipFlop)
    (:A
      _)
    (:B
      _))
  (for _array_element (Variables|Default|GetLights_A)
    (Rendering|SetVisibility _array_element _isa false))
  (for _array_element_2 (Variables|Default|GetLights_B)
    (Rendering|SetVisibility _array_element_2 (not _isa) false)))

(event EventBeginPlay
  (Utilities|Time|SetTimerbyEvent (delegate Custom|ChangeLights) 1.0 true)
  (bind _lights (CallFunction|GetLights))
  (for _index (range 0 (- (/ (Utilities|Array|Length _lights) 2) 1))
    (Utilities|Array|Add (Variables|Default|GetLights_A) (Utilities|Array|Get(acopy) _lights _index)))
  (for _array_element _lights
    (if (not (Utilities|Array|ContainsItem (Variables|Default|GetLights_A) _array_element))
      (Utilities|Array|Add (Variables|Default|GetLights_B) _array_element))))

(fn ConstructionScript)

(fn GetLights
  (for _array_element (CallFunction|GetLightActors)
    (bind _asbp_light_reflector (Utilities|Casting|CastToBP_LightReflector _array_element))
    (Utilities|Array|Add (LocalVariables|GetTemp) (Variables|/Game/Assets/Decos/Muebles/LucesPlataforma1/BP_LightReflector.BP_LightReflector_C|GetSpotLight _asbp_light_reflector)))
  (return (LocalVariables|GetTemp)))

(fn GetLightActors
  (return (Utilities|Array|MakeArray (Variables|/Script/Engine.ChildActorComponent|GetChildActor (Variables|Default|GetChildActor3)) (Variables|/Script/Engine.ChildActorComponent|GetChildActor (Variables|Default|GetChildActor1)) (Variables|/Script/Engine.ChildActorComponent|GetChildActor (Variables|Default|GetChildActor)) (Variables|/Script/Engine.ChildActorComponent|GetChildActor (Variables|Default|GetChildActor4)) (Variables|/Script/Engine.ChildActorComponent|GetChildActor (Variables|Default|GetChildActor5)) (Variables|/Script/Engine.ChildActorComponent|GetChildActor (Variables|Default|GetChildActor2)))))