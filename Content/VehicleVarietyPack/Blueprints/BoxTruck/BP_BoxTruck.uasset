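; Box truck vehicle Blueprint that drives itself forward and cuts throttle when another wheeled vehicle is ahead.
; A Tick-driven Delay refreshes a forward visibility line trace from the Box component about every quarter second, flagging hits on WheeledVehicle actors.
; Each tick, that flag sets throttle to zero or full, with no steering or brake input.
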(event EventTick
  (params (DeltaSeconds :type Float%20%28single-precision%29))
  (bind _vehiclemovement (Variables|Default|GetVehicleMovement))
  (Utilities|FlowControl|Sequence
    (:then_0
      (Utilities|FlowControl|Delay 0.25)
      (bind _hit (CallFunction|LineTrace 1e+03))
      (Variables|Default|SetHitVehicle? _hit))
    (:then_1
      (if (Variables|Default|GetHitVehicle?)
        (Class|WheeledVehicleMovementComponent|SetThrottleInput _vehiclemovement 0.0)
        (else
          (Class|WheeledVehicleMovementComponent|SetThrottleInput _vehiclemovement 1.0))))))

(fn ConstructionScript)

(fn LineTrace
  (params (Len :type Float%20%28single-precision%29))
  (bind _box (Variables|Default|GetBox))
  (bind _returnvalue (Transformation|GetWorldLocation _box))
  (bind _outhit (Collision|LineTraceByChannel _returnvalue (+ (* (Math|Vector|GetForwardVector _box) Len) _returnvalue) "TraceTypeQuery1" false 0 "None"))
  (Utilities|Casting|CastToWheeledVehicle (.HitActor (Collision|BreakHitResult _outhit))
    (:then
      (return true))
    (:CastFailed
      (return false))))