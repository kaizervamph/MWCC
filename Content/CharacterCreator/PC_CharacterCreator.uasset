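; Player controller for the character creator that opens its UI and tracks the character's outfit.
; Equip events toggle clothing slots, while a name-keyed SavedMeshes map holds one entry per type with its material set and colors.
; Loading replays saved shapes, equips and colors onto BP_CharacterCreator; deleting updates the CharactersLibrary save and load list.
; Left-click grabs simulating viewer bodies via a physics handle, but the drag-update logic is disconnected.
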(event Custom|EquipNewCloth
  (params (Info :type CC%20Equips%20Struct%20Structure))
  (bind (_mesh _type) (Utilities|Struct|BreakCCEquipsStruct Info))
  (switch Utilities|FlowControl|Switch|SwitchonClothTypesEnum _type
    (:NewEnumerator0
      (if (== _mesh (.Mesh (Utilities|Struct|BreakCCEquipsStruct (Variables|Default|GetEquipShoes))))
        (Variables|Default|SetEquipShoes "")
        (else
          (Variables|Default|SetEquipShoes Info))))
    (:NewEnumerator1
      (if (== _mesh (.Mesh (Utilities|Struct|BreakCCEquipsStruct (Variables|Default|GetEquipCompleteSet))))
        (Variables|Default|SetEquipCompleteSet "")
        (else
          (Variables|Default|SetEquipCompleteSet Info)
          (CallFunction|EquipNewCloth (Utilities|Struct|MakeCCEquipsStruct 0 "NewEnumerator2")))))
    (:NewEnumerator2
      (if (== _mesh (.Mesh (Utilities|Struct|BreakCCEquipsStruct (Variables|Default|GetEquipPants))))
        (Variables|Default|SetEquipPants "")
        (else
          (Variables|Default|SetEquipPants Info)
          (Variables|Default|SetEquipCompleteSet ""))))
    (:NewEnumerator3
      (if (== _mesh (.Mesh (Utilities|Struct|BreakCCEquipsStruct (Variables|Default|GetEquipJacket))))
        (Variables|Default|SetEquipJacket "")
        (else
          (Variables|Default|SetEquipJacket Info))))
    (:NewEnumerator4
      (if (== _mesh (.Mesh (Utilities|Struct|BreakCCEquipsStruct (Variables|Default|GetEquipHair))))
        (Variables|Default|SetEquipHair "")
        (else
          (Variables|Default|SetEquipHair Info))))
    (:NewEnumerator5
      (if (== _mesh (.Mesh (Utilities|Struct|BreakCCEquipsStruct (Variables|Default|GetEquipShirt))))
        (Variables|Default|SetEquipShirt "")
        (else
          (Variables|Default|SetEquipShirt Info))))))

(event Custom|SaveNewMesh
  (params (SaveName :type String) (Mesh :type Skeletal%20Mesh%20Object%20Reference) (Type :type ClothTypesEnum%20Enum :default "NewEnumerator0") (Color1 :type Linear%20Color%20Structure) (Color2 :type Linear%20Color%20Structure) (MakeUp :type Texture%202D%20Object%20Reference))
  (bind _find (CallFunction|FindSavedMesh SaveName))
  (if _find
    _
    (else
      (CallFunction|RemoveSavedMeshbyType Type)
      (Utilities|Map|Add (Variables|Default|GetSavedMeshes) SaveName (Utilities|Struct|MakeCCEquipsStruct Mesh Type "(DisplayName_5_4D6A40AA49B6969EF275CD82C993F6A4=\"\",Materials_6_B197DF3349A0DBC8ED12969E041AF393=)" Color1 Color2 MakeUp))))
  (CallFunction|PrintSaved))

(event Custom|PrintSaved)

(event Custom|UpdateSetColor2
  (params (MeshName :type String) (Color :type Linear%20Color%20Structure))
  (bind _find (CallFunction|FindSavedMesh MeshName))
  (if _find
    (bind _structout (Utilities|Struct|SetmembersinCCEquipsStruct (.Value (Utilities|Map|Find (Variables|Default|GetSavedMeshes) MeshName)) Color))
    (Utilities|Map|Remove (Variables|Default|GetSavedMeshes) MeshName)
    (Utilities|Map|Add (Variables|Default|GetSavedMeshes) MeshName _structout)))

(event Custom|UpdateSet
  (params (MeshName :type String) (SetInfo :type Multiple%20Materials%20Struct%20Structure))
  (bind _find (CallFunction|FindSavedMesh MeshName))
  (if _find
    (bind _structout (Utilities|Struct|SetmembersinCCEquipsStruct (.Value (Utilities|Map|Find (Variables|Default|GetSavedMeshes) MeshName)) SetInfo))
    (Utilities|Map|Remove (Variables|Default|GetSavedMeshes) MeshName)
    (Utilities|Map|Add (Variables|Default|GetSavedMeshes) MeshName _structout)))

(event Custom|DeleteSavedCharacter
  (params (SavedCharacter :type Save%20Character%20Struct%20Structure))
  (bind _library (CallFunction|GetCharacterLibrary))
  (Utilities|Array|RemoveItem (Variables|/Game/CharacterCreator/Save/SG_CharactersLibrary.SG_CharactersLibrary_C|GetCharacters _library) SavedCharacter)
  (SaveGame|SaveGametoSlot _library "CharactersLibrary")
  (Variables|Default|SetCharacterName "")
  (Utilities|Platform|CollectGarbage)
  (bind _foundwidgets (Widget|GetAllWidgetsOfClass "/Game/CharacterCreator/WBP_CC_LoadCharacter.WBP_CC_LoadCharacter_C" false))
  (for _array_element _foundwidgets
    (Default|UpdateList _array_element)
    (Variables|/Game/CharacterCreator/WBP_CC_LoadCharacter.WBP_CC_LoadCharacter_C|SetSelectedCharacterToLoad _array_element "")))

(event Custom|UpdateSetColor1
  (params (MeshName :type String) (Color :type Linear%20Color%20Structure))
  (bind _find (CallFunction|FindSavedMesh MeshName))
  (if _find
    (bind _structout (Utilities|Struct|SetmembersinCCEquipsStruct (.Value (Utilities|Map|Find (Variables|Default|GetSavedMeshes) MeshName)) Color))
    (Utilities|Map|Remove (Variables|Default|GetSavedMeshes) MeshName)
    (Utilities|Map|Add (Variables|Default|GetSavedMeshes) MeshName _structout)))

(event Custom|LoadSavedCharacter
  (params (SavedCharacter :type Save%20Character%20Struct%20Structure))
  (bind (_female _name _body _bodyshapes _equips _bodycolor _eyescolor _lipscolor _nailscolor) (Utilities|Struct|BreakSaveCharacterStruct SavedCharacter))
  (Utilities|Map|Clear (Variables|Default|GetSavedMeshes))
  (Utilities|Platform|CollectGarbage)
  (bind _foundwidgets (Widget|GetAllWidgetsOfClass "/Game/CharacterCreator/WBP_CC_LoadCharacter.WBP_CC_LoadCharacter_C" false))
  (for _array_element _foundwidgets
    (Default|ForceClose _array_element))
  (bind _actor (CallFunction|GetCC))
  (Utilities|FlowControl|Sequence
    (:then_0
      (Variables|Default|SetCharacterName _name))
    (:then_1
      (CallFunction|LoadSavedShapes _bodyshapes _actor))
    (:then_2
      (CallFunction|LoadSavedEquips _equips _actor))
    (:then_3
      (CallFunction|LoadSavedColors _actor _bodycolor _eyescolor _lipscolor _nailscolor))))

(event EventBeginPlay
  (bind _returnvalue (UserInterface|CreateWidget "/Game/CharacterCreator/WBP_CharacterCreator.WBP_CharacterCreator_C"))
  (Variables|Default|SetCC _returnvalue)
  (Input|SetInputModeGameandUI self _returnvalue "DoNotLock" false)
  (UserInterface|Viewport|AddtoViewport _returnvalue 0))

(event EventTick
  (params (DeltaSeconds :type Float%20%28single-precision%29)))

(event Input|MouseEvents|LeftMouseButton
  (params (Key :type Key%20Structure :default "None"))
  (bind _array (Utilities|Array|MakeArray "ObjectTypeQuery4"))
  (bind _hitresult (Class|PlayerController|GetHitResultUnderCursorforObjects _array true))
  (bind (_bblockinghit _binitialoverlap _time _distance _location _impactpoint _normal _impactnormal _physmat _hitactor _hitcomponent _hitbonename) (Collision|BreakHitResult _hitresult))
  (:Pressed
    (Variables|Default|SetMouseLeft true)
    (bind _asbp_cc_character_viewer (Utilities|Casting|CastToBP_CC_CharacterViewer _hitactor))
    (if (Physics|IsSimulatingPhysics _hitcomponent _hitbonename)
      (bind _ascomponente_de_malla_del_esqueleto (Utilities|Casting|CastToSkeletalMeshComponent _hitcomponent))
      (Variables|Default|SetPhysics%20Handle (Variables|/Game/CharacterCreator/BP_CC_CharacterViewer.BP_CC_CharacterViewer_C|GetPhysicsHandle _asbp_cc_character_viewer))
      (Physics|Components|PhysicsHandle|GrabComponentatLocationwithRotation (Variables|/Game/CharacterCreator/BP_CC_CharacterViewer.BP_CC_CharacterViewer_C|GetPhysicsHandle _asbp_cc_character_viewer) _ascomponente_de_malla_del_esqueleto _hitbonename _impactpoint (Transformation|GetSocketRotation _ascomponente_de_malla_del_esqueleto _hitbonename))))
  (:Released
    (Variables|Default|SetMouseLeft false)
    (bind _physics_handle (Variables|Default|GetPhysics%20Handle)
      (:then
        (Physics|Components|PhysicsHandle|ReleaseComponent _physics_handle))
      (:else))))

(fn ConstructionScript)

(fn GetEquipbyType
  (params (Type :type ClothTypesEnum%20Enum :default "NewEnumerator0")))

(fn SetEquipbyType
  (params (Type :type ClothTypesEnum%20Enum :default "NewEnumerator0") (Cloth :type CC%20Equips%20Struct%20Structure))
  (return false))

(fn FindSavedMesh
  (params (SaveName :type String))
  (bind _savedmeshes (Variables|Default|GetSavedMeshes))
  (bind (_value _returnvalue) (Utilities|Map|Find _savedmeshes SaveName))
  (return _returnvalue _value))

(fn RemoveSavedMeshbyType
  (params (Type :type ClothTypesEnum%20Enum :default "NewEnumerator0"))
  (bind _savedmeshes (Variables|Default|GetSavedMeshes))
  (bind _keys (Utilities|Map|Keys _savedmeshes))
  (for _array_element _keys
    (if (Utilities|Enum|Equal(Enum) (.Type (Utilities|Struct|BreakCCEquipsStruct (.Value (Utilities|Map|Find _savedmeshes _array_element)))) Type)
      (Utilities|Array|Add (LocalVariables|GetTemp) _array_element)))
  (for _array_element_2 (LocalVariables|GetTemp)
    (Utilities|Map|Remove (Variables|Default|GetSavedMeshes) _array_element_2))
  (return true))

(fn FindSavedMeshbyType
  (params (Type :type ClothTypesEnum%20Enum :default "NewEnumerator0"))
  (bind _savedmeshes (Variables|Default|GetSavedMeshes))
  (bind _keys (Utilities|Map|Keys _savedmeshes))
  (for _array_element _keys
    (if (Utilities|Enum|Equal(Enum) (.Type (Utilities|Struct|BreakCCEquipsStruct (.Value (Utilities|Map|Find _savedmeshes _array_element)))) Type)
      (return (.ReturnValue (Utilities|Map|Find _savedmeshes _array_element)) (.Value (Utilities|Map|Find _savedmeshes _array_element)))))
  (return false ""))

(fn GetCC
  (bind _outactors (Actor|GetAllActorsOfClass "/Game/CharacterCreator/BP_CharacterCreator.BP_CharacterCreator_C"))
  (return (Utilities|Array|Get(acopy) _outactors)))

(fn LoadSavedShapes
  (params (Shapes :type Map%20of%20Strings%20to%20Float%20%28single-precision%29s) (CCactor :type BP%20Character%20Creator%20Object%20Reference))
  (bind _keys (Utilities|Map|Keys Shapes))
  (for _array_element _keys
    (Default|ChangeShape CCactor (Utilities|Struct|MakeCCShapesStruct (Utilities|String|StringToName _array_element)) (.Value (Utilities|Map|Find Shapes _array_element))))
  (return true))

(fn LoadSavedEquips
  (params (Equips :type Array%20of%20CC%20Equips%20Struct%20Structures) (CCactor :type BP%20Character%20Creator%20Object%20Reference))
  (bind (_body _hair _cloth _shoes _jacket _pants _shirt) (Default|GetBodyMeshes CCactor))
  (for _array_element Equips
    (bind (_rowname _fila_de_salida) (CallFunction|GetRowNameforCloth (.Mesh (Utilities|Struct|BreakCCEquipsStruct _array_element))))
    (Default|ChangeCloth CCactor (.Type (Utilities|Struct|BreakCCEquipsStruct _array_element)) _rowname (Utilities|Array|FindItem (Utilities|Struct|BreakClothStruct _fila_de_salida) (.Set (Utilities|Struct|BreakCCEquipsStruct _array_element))))
    (Default|ChangeClothMaterial CCactor (Utilities|Select :Index (.Type (Utilities|Struct|BreakCCEquipsStruct _array_element)) :NewEnumerator0 _shoes :NewEnumerator1 _cloth :NewEnumerator2 _pants :NewEnumerator3 _jacket :NewEnumerator4 _hair :NewEnumerator5 _shirt :NewEnumerator6 0 :NewEnumerator7 0) (.Set (Utilities|Struct|BreakCCEquipsStruct _array_element)) _fila_de_salida)
    (Utilities|FlowControl|Sequence
      (:then_0
        (Default|ChangeClothColor CCactor (.Color (Utilities|Struct|BreakCCEquipsStruct _array_element)) (.Type (Utilities|Struct|BreakCCEquipsStruct _array_element))))
      (:then_1
        (Default|ChangeClothColor CCactor (.Color2 (Utilities|Struct|BreakCCEquipsStruct _array_element)) (.Type (Utilities|Struct|BreakCCEquipsStruct _array_element)) 1))))
  (return true))

(fn LoadSavedColors
  (params (CCactor :type BP%20Character%20Creator%20Object%20Reference) (Body :type Linear%20Color%20Structure) (Eyes :type Linear%20Color%20Structure) (Lips :type Linear%20Color%20Structure) (Nails :type Linear%20Color%20Structure))
  (Default|ChangeSkinColor CCactor Body)
  (Default|ChangeEyesColor CCactor Eyes)
  (Default|ChangeLipsColor CCactor Lips)
  (Default|ChangeNailsColor CCactor Nails)
  (return true))