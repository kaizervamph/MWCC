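; Character creator stage actor that previews and customizes a character held in a child BP_CC_CharacterViewer.
; Exposes functions for morph-target shapes, animation, hair, DT_Cloth outfits with random material sets, and colors via material parameters or dynamic instances; eyelash color is an empty stub.
; Blends between child BP_CC_Camera views per body area or a free pawn view, with wheel zoom.
; An input axis rotates the character unless the controller's MouseLeft is set.
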(event Custom|RotateCharacter
  (params (Value :type Float%20%28single-precision%29))
  (bind _aspc_character_creator (Utilities|Casting|CastToPC_CharacterCreator (Game|GetPlayerController 0)))
  (if (not (Variables|/Game/CharacterCreator/PC_CharacterCreator.PC_CharacterCreator_C|GetMouseLeft _aspc_character_creator))
    (Transformation|AddLocalRotation (Variables|Default|GetBody1) (Math|Rotator|MakeRotator 0.0 0.0 (* Value 3.0)) false false)))

(event EventBeginPlay
  (CallFunction|ChangeCamera "Body" 0.0))

(event Collision|EventActorBeginOverlap
  (params (OtherActor :type Actor%20Object%20Reference)))

(event EventTick
  (params (DeltaSeconds :type Float%20%28single-precision%29)))

(event Input|MouseEvents|MouseWheelDown
  (params (Key :type Key%20Structure))
  (:Pressed
    (CallFunction|ChangeCameraZoom 5.0)))

(event Input|MouseEvents|MouseWheelUp
  (params (Key :type Key%20Structure))
  (:Pressed
    (CallFunction|ChangeCameraZoom -5.0)))

(fn ConstructionScript
  (CallFunction|ChangeHair))

(fn GetMorphoTargets
  (return (Class|SkeletalMesh|GetAllMorphTargetNames (Variables|/Script/Engine.SkinnedMeshComponent|GetSkeletalMesh (.Body (CallFunction|GetBodyMeshes))))))

(fn SetMorphoTarget
  (params (MorphTargetName :type Name) (Value :type Float%20%28single-precision%29))
  (Components|SkeletalMesh|SetMorphTarget (.Body (CallFunction|GetBodyMeshes)) MorphTargetName Value true)
  (return true))

(fn GetMorphoTarget
  (params (MorphTargetName :type Name))
  (return (Class|SkeletalMeshComponent|GetMorphTarget (.Body (CallFunction|GetBodyMeshes)) MorphTargetName)))

(fn ChangeSkinColor
  (params (Color :type Linear%20Color%20Structure))
  (Rendering|Material|SetVectorParameterValueonMaterials (.Body (CallFunction|GetBodyMeshes)) "SkinColor" (Math|Conversions|ToVector(LinearColor) Color))
  (return true))

(fn ChangeCloth
  (params (ClothType :type ClothTypesEnum%20Enum :default "NewEnumerator0") (ClothRowName :type Name))
  (bind (_body _hair _cloth _shoes) (CallFunction|GetBodyMeshes))
  (bind _returnvalue (Utilities|Select :Index ClothType :NewEnumerator0 _shoes :NewEnumerator1 _cloth))
  (bind _returnvalue_2 (Utilities|GetDataTableRow "/Game/ProceduralGeneration/DT_Cloth.DT_Cloth" ClothRowName)
    (:then
      (Class|SkinnedMeshComponent|SetSkeletalMesh _returnvalue (.Mesh (Utilities|Struct|BreakClothStruct _returnvalue_2)) false)
      (CallFunction|ChangeClothMaterial _returnvalue (.OutItem (Utilities|Array|Random (.Materials (Utilities|Struct|BreakClothStruct _returnvalue_2)))))
      (return true))
    (:RowNotFound
      (return false))))

(fn ClearAllMorphoTargets
  (Class|SkeletalMeshComponent|ClearMorphTargets (.Body (CallFunction|GetBodyMeshes)))
  (return true))

(fn ChangeClothColor
  (params (Color :type Linear%20Color%20Structure) (ClothType :type ClothTypesEnum%20Enum :default "NewEnumerator0"))
  (bind (_body _hair _cloth _shoes) (CallFunction|GetBodyMeshes))
  (Rendering|Material|SetVectorParameterValueonMaterials (Utilities|Select :Index ClothType :NewEnumerator0 _shoes :NewEnumerator1 _cloth) "Color" (Math|Conversions|ToVector(LinearColor) Color))
  (return true))

(fn ChangeAnimation
  (params (NewAnimToPlay :type Animation%20Asset%20Object%20Reference))
  (Components|Animation|PlayAnimation (Variables|Default|GetBody1) NewAnimToPlay true)
  (return true))

(fn ChangePoleVisibility
  (params (Value :type Boolean))
  (Rendering|SetVisibility (Variables|Default|GetPole_Base_Visor) Value false)
  (return true))

(fn ChangeCamera
  (params (Type :type String) (BlendTime :type Float%20%28single-precision%29))
  (if (Utilities|Enum|Equal(Enum) Type "Free")
    (Variables|Default|SetCurrentCamera "Free")
    (Variables|Default|SetCurrentCameraActor 0)
    (Game|Player|SetViewTargetwithBlend (Game|GetPlayerController 0) (Game|Player|GetPlayerPawn 0) 0.0 "VTBlend_Linear" 0.0 false)
    (return true)
    (else
      (for _array_element (CallFunction|GetCameras)
        (if (Utilities|Enum|Equal(Enum) (Variables|/Game/CharacterCreator/BP_CC_Camera.BP_CC_Camera_C|GetType _array_element) Type)
          (Variables|Default|SetCurrentCamera (Variables|/Game/CharacterCreator/BP_CC_Camera.BP_CC_Camera_C|GetType _array_element))
          (Variables|Default|SetCurrentCameraActor _array_element)
          (Default|ResetArmPosition _array_element)
          (Game|Player|SetViewTargetwithBlend (Game|GetPlayerController 0) _array_element BlendTime "VTBlend_Linear" 0.0 true)
          (return true)))
      (return false))))

(fn GetCameras
  (return (Utilities|Array|MakeArray (.AsBP%20CC%20Camera (Utilities|Casting|CastToBP_CC_Camera (Variables|/Script/Engine.ChildActorComponent|GetChildActor (Variables|Default|GetChildActor_Head)))) (.AsBP%20CC%20Camera (Utilities|Casting|CastToBP_CC_Camera (Variables|/Script/Engine.ChildActorComponent|GetChildActor (Variables|Default|GetChildActor_Chest)))) (.AsBP%20CC%20Camera (Utilities|Casting|CastToBP_CC_Camera (Variables|/Script/Engine.ChildActorComponent|GetChildActor (Variables|Default|GetChildActor_Pelvis)))) (.AsBP%20CC%20Camera (Utilities|Casting|CastToBP_CC_Camera (Variables|/Script/Engine.ChildActorComponent|GetChildActor (Variables|Default|GetChildActor_Body)))) (.AsBP%20CC%20Camera (Utilities|Casting|CastToBP_CC_Camera (Variables|/Script/Engine.ChildActorComponent|GetChildActor (Variables|Default|GetChildActor_Feet)))))))

(fn ChangeCameraZoom
  (params (Value :type Float%20%28single-precision%29))
  (if (Utilities|Enum|NotEqual(Enum) (Variables|Default|GetCurrentCamera) "Free")
    (for _array_element (CallFunction|GetCameras)
      (if (Utilities|Enum|Equal(Enum) (Variables|/Game/CharacterCreator/BP_CC_Camera.BP_CC_Camera_C|GetType _array_element) (Variables|Default|GetCurrentCamera))
        (Default|CameraZoom _array_element Value)
        (return true)))
    (else
      (return false))))

(fn GetBodyMeshes
  (bind _asbp_cc_character_viewer (Utilities|Casting|CastToBP_CC_CharacterViewer (Variables|/Script/Engine.ChildActorComponent|GetChildActor (Variables|Default|GetChildActor_Character))))
  (return (Variables|/Script/Engine.Character|GetMesh _asbp_cc_character_viewer) (Variables|/Game/CharacterCreator/BP_CC_CharacterViewer.BP_CC_CharacterViewer_C|GetHair _asbp_cc_character_viewer) (Variables|/Game/CharacterCreator/BP_CC_CharacterViewer.BP_CC_CharacterViewer_C|GetCloth _asbp_cc_character_viewer) (Variables|/Game/CharacterCreator/BP_CC_CharacterViewer.BP_CC_CharacterViewer_C|GetShoes _asbp_cc_character_viewer)))

(fn ChangeClothMaterial
  (params (Component :type Primitive%20Component%20Object%20Reference) (Material :type Multiple%20Materials%20Struct%20Structure%20%28by%20ref%29))
  (for (_array_element _array_index) (.Materials (Utilities|Struct|BreakMultipleMaterialsStruct Material))
    (Rendering|Material|SetMaterial Component _array_index _array_element))
  (return true))

(fn ChangeEyesColor
  (params (NewColor :type Linear%20Color%20Structure))
  (bind _body (CallFunction|GetBodyMeshes))
  (bind _returnvalue (Rendering|Material|CreateDynamicMaterialInstance _body 7 (Rendering|Material|GetMaterial _body 7) "None" :!class /Script/Engine.PrimitiveComponent))
  (LocalVariables|SetDynMat _returnvalue)
  (Rendering|Material|SetVectorParameterValue (LocalVariables|GetDynMat) "Diffuse Color" NewColor :!class /Script/Engine.MaterialInstanceDynamic)
  (Rendering|Material|SetMaterial _body 7 (LocalVariables|GetDynMat))
  (return true))

(fn ChangeEyelashesColor
  (params (NewColor :type Linear%20Color%20Structure)))

(fn ChangeLipsColor
  (params (NewColor :type Linear%20Color%20Structure))
  (bind _body (CallFunction|GetBodyMeshes))
  (bind _returnvalue (Rendering|Material|CreateDynamicMaterialInstance _body 1 (Rendering|Material|GetMaterial _body 1) "None" :!class /Script/Engine.PrimitiveComponent))
  (LocalVariables|SetDynMat _returnvalue)
  (Rendering|Material|SetVectorParameterValue (LocalVariables|GetDynMat) "SkinColor" NewColor :!class /Script/Engine.MaterialInstanceDynamic)
  (Rendering|Material|SetMaterial _body 1 (LocalVariables|GetDynMat))
  (return true))

(fn ChangeHairColor
  (params (NewColor :type Linear%20Color%20Structure))
  (bind _hair (CallFunction|GetBodyMeshes))
  (bind _returnvalue (Rendering|Material|CreateDynamicMaterialInstance _hair 0 (Rendering|Material|GetMaterial _hair 0) "None" :!class /Script/Engine.PrimitiveComponent))
  (LocalVariables|SetDynMat _returnvalue)
  (Rendering|Material|SetVectorParameterValue (LocalVariables|GetDynMat) "Color Gradient A" NewColor :!class /Script/Engine.MaterialInstanceDynamic)
  (Rendering|Material|SetVectorParameterValue (LocalVariables|GetDynMat) "Color Gradient B" NewColor :!class /Script/Engine.MaterialInstanceDynamic)
  (Rendering|Material|SetMaterial _hair 0 (LocalVariables|GetDynMat))
  (return true))

(fn ChangeHair
  (Class|SkinnedMeshComponent|SetSkeletalMesh (.Hair (CallFunction|GetBodyMeshes)) (Variables|Default|GetHairMeshPreview) true))

(fn ChangeShape
  (params (Info :type CC%20Shapes%20Struct%20Structure) (Value :type Float%20%28single-precision%29))
  (Components|SkeletalMesh|SetMorphTarget (.Body (CallFunction|GetBodyMeshes)) (.Shape (Utilities|Struct|BreakCCShapesStruct Info)) Value true)
  (return true))

(fn GetShapeValue
  (params (Info :type CC%20Shapes%20Struct%20Structure))
  (return (Class|SkeletalMeshComponent|GetMorphTarget (.Body (CallFunction|GetBodyMeshes)) (.Shape (Utilities|Struct|BreakCCShapesStruct Info)))))