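; BP_EBS_GameMode is the Easy Building System game mode, set up to react to day and night changes.
; On BeginPlay it finds the first Ultra_Dynamic_Sky actor and binds its sunrise and sunset events to day and night configuration events.
; These call TurnLights off or on, but that event is empty.
; ChangePP is also empty, with disconnected logic for toggling Day- and Night-tagged PostProcessVolumes.
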(event Custom|OnSunset
  (CallFunction|NightConfiguration))

(event Custom|NightConfiguration
  (CallFunction|TurnLights true))

(event Custom|DayConfigurations
  (CallFunction|TurnLights false))

(event Custom|ChangePP
  (params (Day :type Boolean)))

(event Custom|OnSunrise
  (CallFunction|DayConfigurations))

(event Custom|TurnLights
  (params (Value :type Boolean)))

(event EventBeginPlay
  (bind _outactors (Actor|GetAllActorsOfClass "/Game/UltraDynamicSky/Blueprints/Ultra_Dynamic_Sky.Ultra_Dynamic_Sky_C"))
  (bind _output_get (Variables|Default|SetUDS (Utilities|Array|Get(acopy) _outactors)))
  (EventDispatchers|BindEventtoSunset _output_get (delegate Custom|OnSunset))
  (EventDispatchers|BindEventtoSunrise _output_get (delegate Custom|OnSunrise)))

(event EventTick
  (params (DeltaSeconds :type Float%20%28single-precision%29)))

(fn ConstructionScript)