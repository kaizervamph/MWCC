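; Base spectator pawn for the Easy Building System, providing free-camera movement and look.
; On possession it binds to the player controller's time-speed change and sets its CustomTimeDilation to the inverse, offsetting game speed.
; Forward and strafe input also triggers LightVisibility on every lamp building, found via GetAllActorsOfClass on each input.
; When the view target is an employee, mouse X rotates that employee's third-person camera and mouse Y is ignored.
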(event Custom|OnTimeSpeedChange
  (params (TimeSpeed :type Integer))
  (bind _returnvalue (Math|Float|MakeLiteralFloat 1.0))
  (bind _returnvalue_2 (Math|Conversions|ToFloat(Integer) TimeSpeed))
  (bind _returnvalue_3 (/ _returnvalue _returnvalue_2))
  (Variables|Default|SetCustomTimeDilation (select (<= _returnvalue_3 0.0) 1.0 _returnvalue_3)))

(event Custom|LightsHidden
  (bind _outactors (Actor|GetAllActorsOfClass "/Game/EasyBuildingSystem/Blueprints/BuildingObjects/Placeable/BP_EBS_Building_Lamp.BP_EBS_Building_Lamp_C"))
  (for _array_element _outactors
    (Default|LightVisibility _array_element)))

(event EventBeginPlay)

(event EventPossessed
  (params (NewController :type Controller%20Object%20Reference))
  (bind _asbp_ebs_player_controller (Utilities|Casting|CastToBP_EBS_PlayerController NewController))
  (bind _output_get (Variables|Default|SetPC _asbp_ebs_player_controller))
  (EventDispatchers|BindEventtoOnChangeTimeSpeed _output_get (delegate Custom|OnTimeSpeedChange)))

(event Input|AxisEvents|InputAxisMoveForward
  (params (AxisValue :type Float%20%28single-precision%29))
  (if (!= AxisValue 0.0)
    (CallFunction|LightsHidden)
    (Pawn|Input|AddMovementInput (Math|Vector|GetForwardVector (Pawn|GetControlRotation :!class /Script/Engine.Pawn)) AxisValue false)))

(event Input|AxisEvents|InputAxisMoveRight
  (params (AxisValue :type Float%20%28single-precision%29))
  (if (!= AxisValue 0.0)
    (CallFunction|LightsHidden)
    (Pawn|Input|AddMovementInput (Math|Vector|GetRightVector (Pawn|GetControlRotation :!class /Script/Engine.Pawn)) AxisValue false)))

(event Input|AxisEvents|InputAxisMoveUp
  (params (AxisValue :type Float%20%28single-precision%29))
  (Class|DefaultPawn|MoveUpWorld AxisValue))

(event Input|MouseEvents|MouseX
  (params (AxisValue :type Float%20%28single-precision%29))
  (bind _asbp_employees_base (Utilities|Casting|CastToBP_EmployeesBase (Pawn|GetViewTarget (Game|GetPlayerController 0)))
    (:then
      (Default|RotateTPcamera _asbp_employees_base AxisValue))
    (:CastFailed
      (Pawn|Input|AddControllerYawInput AxisValue))))

(event Input|MouseEvents|MouseY
  (params (AxisValue :type Float%20%28single-precision%29))
  (Utilities|Casting|CastToBP_EmployeesBase (Pawn|GetViewTarget (Game|GetPlayerController 0))
    (:CastFailed
      (bind _result (Math|Float|NegateFloat AxisValue)
        (:%20%20
          (Pawn|Input|AddControllerPitchInput _result))))))

(fn ConstructionScript)