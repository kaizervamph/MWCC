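; A placeable Easy Building System bench that exposes a single sit socket for users.
; The construction script copies the sockets from GetSockets into FreeSockets, and GetFreeSocket returns the first entry's world transform with a found flag.
; Each tick, if the first user is an employee, it draws that employee's name above the bench as debug text.
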(event EventBeginPlay
  (|CallParentFunction) ; This node is disabled and will not be called.\nDrag off pins to build functionality.
)

(event Collision|EventActorBeginOverlap
  (params (OtherActor :type Actor%20Object%20Reference)))

(event EventTick
  (params (DeltaSeconds :type Float%20%28single-precision%29))
  (bind _users (Variables|Default|GetUsers))
  (if (Utilities|Array|IsValidIndex _users)
    (bind _asbp_employees_base (Utilities|Casting|CastToBP_EmployeesBase (Utilities|Array|Get(acopy) _users)))
    (Utilities|IsValid _asbp_employees_base
      (:Is%20Valid
        (Rendering|Debug|DrawDebugString (+ (Transformation|GetActorLocation) "0, 0,50.000000") (.Name (Utilities|Struct|BreakProceduralCharacterStruct (Variables|/Game/Core/BP_EmployeesBase.BP_EmployeesBase_C|GetCharacterInfo _asbp_employees_base))) 0 "(R=1.000000,G=1.000000,B=1.000000,A=1.000000)" 0.001)))))

(fn ConstructionScript
  (|CallParentFunction)
  (for _array_element (CallFunction|GetSockets)
    (Utilities|IsValid _array_element
      (:Is%20Valid
        (Utilities|Array|AddUnique (Variables|Default|GetFreeSockets) _array_element)))))

(fn GetFreeSocket
  (bind _freesockets (Variables|Default|GetFreeSockets))
  (bind _output (Utilities|Array|Get(acopy) _freesockets))
  (if (Utilities|Array|IsValidIndex _freesockets)
    (Utilities|IsValid _output
      (:Is%20Valid
        (return (Transformation|GetWorldLocation _output) (Transformation|GetWorldRotation _output) _output true))
      (:Is%20Not%20Valid
        _)))
  (return "0, 0, 0" "0, 0, 0" 0 false))

(fn GetSockets
  (return (Utilities|Array|MakeArray (Variables|Default|GetSit_Socket))))