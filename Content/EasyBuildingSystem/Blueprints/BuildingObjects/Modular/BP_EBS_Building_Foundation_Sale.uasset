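; Modular foundation piece for the Easy Building System that carries a buy widget, apparently marking it as a foundation for sale.
; On BeginPlay it passes itself to WBP_BuyFoundation, and each tick turns the widget toward the player's view target.
; Clicking applies the controller's selected floor paint through a dynamic material instance, or destroys the piece in delete mode.
; The construction script reapplies stored paint, and hover highlighting uses custom depth.
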(event OnClicked(StaticMesh)
  (params (TouchedComponent :type Primitive%20Component%20Object%20Reference) (ButtonPressed :type Key%20Structure :default "None"))
  (bind _asbp_ebs_player_controller (Utilities|Casting|CastToBP_EBS_PlayerController (Game|GetPlayerController 0)))
  (if (Variables|/Game/EasyBuildingSystem/Blueprints/Game/BP_EBS_PlayerController.BP_EBS_PlayerController_C|GetBuildPaintActive _asbp_ebs_player_controller)
    (if (Utilities|Enum|Equal(Enum) (Variables|/Game/EasyBuildingSystem/Blueprints/Game/BP_EBS_PlayerController.BP_EBS_PlayerController_C|GetBuildPaintTypeSelected _asbp_ebs_player_controller) "Floor")
      (CallFunction|SetPaintConfig (.ParameterName (Utilities|Struct|BreakBuildPaintingParamsStruct (Variables|/Game/EasyBuildingSystem/Blueprints/Game/BP_EBS_PlayerController.BP_EBS_PlayerController_C|GetPaintSelected _asbp_ebs_player_controller))) (.Material (Utilities|Struct|BreakBuildPaintingParamsStruct (Variables|/Game/EasyBuildingSystem/Blueprints/Game/BP_EBS_PlayerController.BP_EBS_PlayerController_C|GetPaintSelected _asbp_ebs_player_controller)))))
    (elif (Variables|/Game/EasyBuildingSystem/Blueprints/Game/BP_EBS_PlayerController.BP_EBS_PlayerController_C|GetDelete? _asbp_ebs_player_controller)
      (CallFunction|CompleteDestruction(Multicast)))))

(event Custom|SetPaintConfig
  (params (PaintParams :type Array%20of%20Paint%20Parameter%20Struct%20Structures) (PaintMaterial :type Material%20Interface%20Object%20Reference))
  (Variables|Default|SetPaintParams PaintParams)
  (Variables|Default|SetPaintMaterial PaintMaterial)
  (bind _returnvalue (Rendering|Material|CreateDynamicMaterialInstance (Variables|Default|GetPaintMaterial) "None" "None" :!class /Script/Engine.KismetMaterialLibrary))
  (Variables|Default|SetDynMat _returnvalue)
  (for _array_element (Variables|Default|GetPaintParams)
    (bind _dynmat (Variables|Default|GetDynMat)
      (:then
        (Rendering|Material|SetVectorParameterValue _dynmat (.ParameterName (Utilities|Struct|BreakPaintParameterStruct _array_element)) (.Value (Utilities|Struct|BreakPaintParameterStruct _array_element)) :!class /Script/Engine.MaterialInstanceDynamic))
      (:else)))
  (Rendering|Material|SetMaterial (Variables|Default|GetStaticMesh) 0 (Variables|Default|GetDynMat)))

(event Custom|HoverHighlight
  (params (Value :type Boolean))
  (Rendering|SetRenderCustomDepth (Variables|Default|GetStaticMesh) Value))

(event EventBeginPlay
  (bind _aswbp_buy_foundation (Utilities|Casting|CastToWBP_BuyFoundation (UserInterface|GetWidget (Variables|Default|GetWidget))))
  (Variables|/Game/EasyBuildingSystem/Blueprints/BuildingObjects/Modular/WBP_BuyFoundation.WBP_BuyFoundation_C|SetFoundationRef _aswbp_buy_foundation self))

(event EventTick
  (params (DeltaSeconds :type Float%20%28single-precision%29))
  (Transformation|SetRelativeRotation (Variables|Default|GetWidget) (Math|Rotator|FindLookatRotation (Transformation|GetActorLocation) (Transformation|GetActorLocation (Pawn|GetViewTarget (Game|GetPlayerController 0)))) false false))

(fn ConstructionScript
  (|CallParentFunction)
  (CallFunction|SetPaintConfig (Variables|Default|GetPaintParams) (Variables|Default|GetPaintMaterial)))