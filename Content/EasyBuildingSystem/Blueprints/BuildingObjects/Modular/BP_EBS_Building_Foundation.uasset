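; Modular foundation piece for the Easy Building System that the player can repaint or delete by clicking.
; In paint mode with "Floor" selected, cursor hover moves a custom-depth highlight to this foundation and a click applies the controller's selected paint.
; Painting creates a dynamic material instance with vector parameters, also rebuilt from stored settings in the construction script.
; Outside paint mode, a click with Delete active calls the destruction multicast.
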(event OnBeginCursorOver(StaticMesh)
  (params (TouchedComponent :type Primitive%20Component%20Object%20Reference))
  (bind _asbp_ebs_player_controller (Utilities|Casting|CastToBP_EBS_PlayerController (Game|GetPlayerController 0)))
  (if (Variables|/Game/EasyBuildingSystem/Blueprints/Game/BP_EBS_PlayerController.BP_EBS_PlayerController_C|GetBuildPaintActive _asbp_ebs_player_controller)
    (if (Utilities|Enum|Equal(Enum) (Variables|/Game/EasyBuildingSystem/Blueprints/Game/BP_EBS_PlayerController.BP_EBS_PlayerController_C|GetBuildPaintTypeSelected _asbp_ebs_player_controller) "Floor")
      (CallFunction|Hover))))

(event OnClicked(StaticMesh)
  (params (TouchedComponent :type Primitive%20Component%20Object%20Reference) (ButtonPressed :type Key%20Structure))
  (bind _asbp_ebs_player_controller (Utilities|Casting|CastToBP_EBS_PlayerController (Game|GetPlayerController 0)))
  (if (Variables|/Game/EasyBuildingSystem/Blueprints/Game/BP_EBS_PlayerController.BP_EBS_PlayerController_C|GetBuildPaintActive _asbp_ebs_player_controller)
    (if (Utilities|Enum|Equal(Enum) (Variables|/Game/EasyBuildingSystem/Blueprints/Game/BP_EBS_PlayerController.BP_EBS_PlayerController_C|GetBuildPaintTypeSelected _asbp_ebs_player_controller) "Floor")
      (CallFunction|SetPaintConfig (.ParameterName (Utilities|Struct|BreakBuildPaintingParamsStruct (Variables|/Game/EasyBuildingSystem/Blueprints/Game/BP_EBS_PlayerController.BP_EBS_PlayerController_C|GetPaintSelected _asbp_ebs_player_controller))) (.Material (Utilities|Struct|BreakBuildPaintingParamsStruct (Variables|/Game/EasyBuildingSystem/Blueprints/Game/BP_EBS_PlayerController.BP_EBS_PlayerController_C|GetPaintSelected _asbp_ebs_player_controller)))))
    (elif (Variables|/Game/EasyBuildingSystem/Blueprints/Game/BP_EBS_PlayerController.BP_EBS_PlayerController_C|GetDelete? _asbp_ebs_player_controller)
      (CallFunction|CompleteDestruction(Multicast)))))

(event Custom|SetPaintConfig
  (params (PaintParams :type Array%20of%20Paint%20Parameter%20Struct%20Structures) (PaintMaterial :type Material%20Interface%20Object%20Reference))
  (Variables|Default|SetPaintParams PaintParams)
  (Variables|Default|SetPaintMaterial PaintMaterial)
  (bind _returnvalue (Rendering|Material|CreateDynamicMaterialInstance (Variables|Default|GetPaintMaterial) "None" "None" :!class /Script/Engine.KismetMaterialLibrary))
  (Variables|Default|SetDynMat _returnvalue)
  (for _array_element (Variables|Default|GetPaintParams)
    (bind _dynmat (Variables|Default|GetDynMat)
      (:then
        (Rendering|Material|SetVectorParameterValue _dynmat (.ParameterName (Utilities|Struct|BreakPaintParameterStruct _array_element)) (.Value (Utilities|Struct|BreakPaintParameterStruct _array_element)) :!class /Script/Engine.MaterialInstanceDynamic))
      (:else)))
  (Rendering|Material|SetMaterial (Variables|Default|GetStaticMesh) 0 (Variables|Default|GetDynMat)))

(event Custom|Hover
  (bind _outactors (Actor|GetAllActorsOfClass "BP_EBS_Building_Foundation_C"))
  (for _array_element _outactors
    (CallFunction|HoverHighlight _array_element false))
  (CallFunction|HoverHighlight true))

(event Custom|HoverHighlight
  (params (Value :type Boolean))
  (Rendering|SetRenderCustomDepth (Variables|Default|GetStaticMesh) Value))

(fn ConstructionScript
  (|CallParentFunction)
  (CallFunction|SetPaintConfig (Variables|Default|GetPaintParams) (Variables|Default|GetPaintMaterial)))