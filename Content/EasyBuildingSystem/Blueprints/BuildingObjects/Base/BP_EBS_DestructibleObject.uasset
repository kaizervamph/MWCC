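; Base destructible object for the Easy Building System that shatters as soon as it spawns, then cleans itself up.
; The construction script assigns the destructible mesh to the DestructibleComponent.
; BeginPlay applies radius damage at the actor's location to break it, disables collision after a short delay, and sets a timer intended to destroy the actor.
; An ApplyMaterials event sets materials on the component's slots.
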(event Custom|ApplyMaterials
  (params (Material :type Array%20of%20Material%20Interface%20Object%20References))
  (for (_ _array_index) Material
    (Rendering|Material|SetMaterial (Variables|Default|GetDestructibleComponent) _array_index "/Engine/EngineDebugMaterials/VertexColorViewMode_RedOnly.VertexColorViewMode_RedOnly")))

(event EventBeginPlay
  ;[1 1 1] Destruct destructible component and destroy actor after delay.
  (Class|DestructibleComponent|ApplyRadiusDamage (Variables|Default|GetDestructibleComponent) 1e+02 (Transformation|GetActorLocation) 0.0 1e+03 false)
  (Utilities|Time|SetTimerbyEvent (EventDispatchers|CreateEvent :!event K2DestroyActor) 6.0)
  (Utilities|FlowControl|Delay 3.0)
  (Collision|SetActorEnableCollision false))

(fn ConstructionScript
  ;[1 1 1] Set destructible mesh.
  (Class|DestructibleComponent|SetDestructibleMesh (Variables|Default|GetDestructibleComponent) (Variables|Default|GetDestructibleMesh)))