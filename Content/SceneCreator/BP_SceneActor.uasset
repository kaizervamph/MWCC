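; Selectable, customizable character placed in the Scene Creator, wrapping a BP_CC_CharacterViewer child actor.
; BeginPlay creates dynamic skin materials, sets Scene_ABP and binds mesh mouse events; clicking makes it the controller's ActorToLoad, highlighted through custom depth.
; Functions edit skin, makeup, eyes, hair and DT_Cloth outfits, clearing conflicting clothing slots.
; ChangeClothColor saves colors through PC_CharacterCreator, unlike selection, which uses PC_SceneCreator.
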(event Custom|SelectAnimation
  (params (ID :type Integer))
  (bind _animation (Variables|SceneAnimation|GetAnimation))
  (if (Utilities|Array|IsValidIndex _animation ID)
    (Variables|Default|SetAnimToPlay (Utilities|Array|Get(acopy) _animation ID))))

(event Custom|SetInteractions
  (bind _asbp_cc_character_viewer (Utilities|Casting|CastToBP_CC_CharacterViewer (Variables|/Script/Engine.ChildActorComponent|GetChildActor (Variables|Default|GetChildActor_Character))))
  (Collision|SetCollisionEnabled (Variables|/Script/Engine.Character|GetMesh _asbp_cc_character_viewer) "QueryOnly")
  (Collision|SetCollisionResponsetoChannel (Variables|/Script/Engine.Character|GetMesh _asbp_cc_character_viewer) "ECC_Visibility" "ECR_Block")
  (EventDispatchers|BindEventtoOnClicked (Variables|/Script/Engine.Character|GetMesh _asbp_cc_character_viewer) (delegate Custom|OnClickedActor))
  (EventDispatchers|BindEventtoOnBeginCursorOver (Variables|/Script/Engine.Character|GetMesh _asbp_cc_character_viewer) (delegate Custom|MouseOn))
  (EventDispatchers|BindEventtoOnEndCursorOver (Variables|/Script/Engine.Character|GetMesh _asbp_cc_character_viewer) (delegate Custom|MouseOff)))

(event Custom|OnClickedActor
  (params (TouchedComponent :type Primitive%20Component%20Object%20Reference) (ButtonPressed :type Key%20Structure :default "None"))
  (bind _self self)
  (bind _aspc_scene_creator (Utilities|Casting|CastToPC_SceneCreator (Game|GetPlayerController 0)))
  (Variables|/Game/SceneCreator/PC_SceneCreator.PC_SceneCreator_C|SetActor%20to%20Load _aspc_scene_creator _self)
  (Development|PrintString (Utilities|String|Append "Selected" (Utilities|GetDisplayName _self)) true true "(R=0.264399,G=1.000000,B=0.000000,A=1.000000)" 5.0))

(event Custom|MouseOn
  (params (TouchedComponent :type Primitive%20Component%20Object%20Reference))
  (bind _aspc_scene_creator (Utilities|Casting|CastToPC_SceneCreator (Game|GetPlayerController 0)))
  (if (!= (Variables|/Game/SceneCreator/PC_SceneCreator.PC_SceneCreator_C|GetActor%20to%20Load _aspc_scene_creator) self)
    (Rendering|SetRenderCustomDepth TouchedComponent true)))

(event Custom|MouseOff
  (params (TouchedComponent :type Primitive%20Component%20Object%20Reference))
  (Rendering|SetRenderCustomDepth TouchedComponent false)
  (Rendering|Material|SetScalarParameterValue "/Game/SurvivalGameKitV2/Materials/MPC_Highlight.MPC_Highlight" "Stencil" 0.0 :!class /Script/Engine.KismetMaterialLibrary))

(event EventBeginPlay
  (bind _body (CallFunction|GetBodyMeshes))
  (Utilities|FlowControl|Sequence
    (:then_0
      (bind (_facemat _torsomat _legsmat _armsmat _lipsmat _nailshandmat _nailsfeetmat) (CallFunction|GetSkinMats))
      (Rendering|Material|SetMaterial _body 0 _facemat)
      (Rendering|Material|SetMaterial _body 3 _torsomat)
      (Rendering|Material|SetMaterial _body 4 _legsmat)
      (Rendering|Material|SetMaterial _body 6 _armsmat)
      (Rendering|Material|SetMaterial _body 1 _lipsmat)
      (Rendering|Material|SetMaterial _body 9 _nailshandmat)
      (Rendering|Material|SetMaterial _body 10 _nailsfeetmat))
    (:then_1
      (bind _asbp_cc_character_viewer (Utilities|Casting|CastToBP_CC_CharacterViewer (Variables|/Script/Engine.ChildActorComponent|GetChildActor (Variables|Default|GetChildActor_Character))))
      (Class|SkeletalMeshComponent|SetAnimClass (Variables|/Script/Engine.Character|GetMesh _asbp_cc_character_viewer) "/Game/SceneCreator/Scene_ABP.Scene_ABP_C"))
    (:then_2
      (CallFunction|SetInteractions))))

(event EventTick
  (params (DeltaSeconds :type Float%20%28single-precision%29))
  (bind _aspc_scene_creator (Utilities|Casting|CastToPC_SceneCreator (Game|GetPlayerController 0)))
  (if (== (Variables|/Game/SceneCreator/PC_SceneCreator.PC_SceneCreator_C|GetActor%20to%20Load _aspc_scene_creator) self)
    (bind _asbp_cc_character_viewer (Utilities|Casting|CastToBP_CC_CharacterViewer (Variables|/Script/Engine.ChildActorComponent|GetChildActor (Variables|Default|GetChildActor_Character))))
    (Rendering|SetRenderCustomDepth (Variables|/Script/Engine.Character|GetMesh _asbp_cc_character_viewer) true)
    (Rendering|Material|SetScalarParameterValue "/Game/SurvivalGameKitV2/Materials/MPC_Highlight.MPC_Highlight" "Stencil" 1.0 :!class /Script/Engine.KismetMaterialLibrary)))

(fn ConstructionScript)

(fn AddNewMesh
  (params (NewMesh :type Skeletal%20Mesh%20Object%20Reference) (Type :type String))
  (bind _returnvalue (AddComponent|AddSkeletalMeshComponent false))
  (Class|SkinnedMeshComponent|SetSkeletalMesh _returnvalue NewMesh true)
  (Utilities|Array|Add (Variables|/Script/Engine.ActorComponent|GetComponentTags _returnvalue) (Utilities|String|StringToName Type))
  (return true _returnvalue))

(fn ClearActor
  (bind _bodymeshcomponent (Variables|Default|GetBodyMeshComponent)
    (:then
      (Components|DestroyComponent _bodymeshcomponent))
    (:else
      _))
  (for _array_element (Variables|Default|GetOtherMeshComponents)
    (Utilities|IsValid _array_element
      (:Is%20Valid
        (Components|DestroyComponent _array_element))))
  (Utilities|Array|Clear (Variables|Default|GetOtherMeshComponents))
  (return true))

(fn ChangeSkinColor
  (params (Value :type Linear%20Color%20Structure))
  (bind _body (CallFunction|GetBodyMeshes))
  (Rendering|Material|SetVectorParameterValue (Variables|Default|GetFaceMat) "SkinColor" Value :!class /Script/Engine.MaterialInstanceDynamic)
  (Rendering|Material|SetMaterial _body 0 (Variables|Default|GetFaceMat))
  (Rendering|Material|SetMaterial _body 3 (Variables|Default|GetTorsoMat))
  (Rendering|Material|SetMaterial _body 4 (Variables|Default|GetLegsMat))
  (Rendering|Material|SetMaterial _body 6 (Variables|Default|GetArmsMat))
  (return true))

(fn ChangeHair
  (params (NewMesh :type Skeletal%20Mesh%20Object%20Reference))
  (bind _hair (CallFunction|GetBodyMeshes))
  (Class|SkinnedMeshComponent|SetSkeletalMesh _hair NewMesh false)
  (Collision|SetCollisionEnabled _hair "NoCollision")
  (Collision|SetCollisionEnabled _hair "QueryAndPhysics"))

(fn GetBodyMeshes
  (bind _asbp_cc_character_viewer (Utilities|Casting|CastToBP_CC_CharacterViewer (Variables|/Script/Engine.ChildActorComponent|GetChildActor (Variables|Default|GetChildActor_Character))))
  (return (Variables|/Script/Engine.Character|GetMesh _asbp_cc_character_viewer) (Variables|/Game/CharacterCreator/BP_CC_CharacterViewer.BP_CC_CharacterViewer_C|GetHair _asbp_cc_character_viewer) (Variables|/Game/CharacterCreator/BP_CC_CharacterViewer.BP_CC_CharacterViewer_C|GetCloth _asbp_cc_character_viewer) (Variables|/Game/CharacterCreator/BP_CC_CharacterViewer.BP_CC_CharacterViewer_C|GetShoes _asbp_cc_character_viewer) (Variables|/Game/CharacterCreator/BP_CC_CharacterViewer.BP_CC_CharacterViewer_C|GetJacket _asbp_cc_character_viewer) (Variables|/Game/CharacterCreator/BP_CC_CharacterViewer.BP_CC_CharacterViewer_C|GetPants _asbp_cc_character_viewer) (Variables|/Game/CharacterCreator/BP_CC_CharacterViewer.BP_CC_CharacterViewer_C|GetShirt _asbp_cc_character_viewer) (Variables|/Game/CharacterCreator/BP_CC_CharacterViewer.BP_CC_CharacterViewer_C|GetUnderwear _asbp_cc_character_viewer)))

(fn ChangeHairColor
  (params (Value :type Linear%20Color%20Structure) (Index :type Integer))
  (bind _hair (CallFunction|GetBodyMeshes))
  (bind _returnvalue (Rendering|Material|CreateDynamicMaterialInstance _hair 0 (Rendering|Material|GetMaterial _hair 0) "None" :!class /Script/Engine.PrimitiveComponent))
  (LocalVariables|SetDynMat _returnvalue)
  (Rendering|Material|SetVectorParameterValue (LocalVariables|GetDynMat) (Utilities|Select :Index Index :Option%200 "Root_Color" :Option%201 "Tip_Color") Value :!class /Script/Engine.MaterialInstanceDynamic)
  (Rendering|Material|SetMaterial _hair 0 (LocalVariables|GetDynMat))
  (return true))

(fn ChangeMakeUp
  (params (Value :type Texture%20Object%20Reference) (Selection :type String))
  (bind _body (CallFunction|GetBodyMeshes))
  (switch string Selection
    (:eyes
      (LocalVariables|SetParamName "Makeup1")
      (LocalVariables|SetClothType "NewEnumerator6"))
    (:face
      (LocalVariables|SetParamName "Makeup2")
      (LocalVariables|SetClothType "NewEnumerator7")))
  (bind _returnvalue (Rendering|Material|CreateDynamicMaterialInstance _body 0 (Rendering|Material|GetMaterial _body 0) "None" :!class /Script/Engine.PrimitiveComponent))
  (LocalVariables|SetDynMat _returnvalue)
  (Rendering|Material|SetTextureParameterValue _returnvalue (LocalVariables|GetParamName) Value)
  (Rendering|Material|SetMaterial _body 0 (LocalVariables|GetDynMat))
  (return true))

(fn ChangeMakeUpColor
  (params (Value :type Linear%20Color%20Structure) (Selection :type String))
  (bind _body (CallFunction|GetBodyMeshes))
  (switch string Selection
    (:eyes
      (LocalVariables|SetParamName "MakeUp1Color1")
      (LocalVariables|SetClothType "NewEnumerator6"))
    (:face
      (LocalVariables|SetParamName "MakeUp2Color1")
      (LocalVariables|SetClothType "NewEnumerator7")))
  (bind _returnvalue (Rendering|Material|CreateDynamicMaterialInstance _body 0 (Rendering|Material|GetMaterial _body 0) "None" :!class /Script/Engine.PrimitiveComponent))
  (LocalVariables|SetDynMat _returnvalue)
  (Rendering|Material|SetVectorParameterValue _returnvalue (LocalVariables|GetParamName) Value :!class /Script/Engine.MaterialInstanceDynamic)
  (Rendering|Material|SetMaterial _body 0 (LocalVariables|GetDynMat)))

(fn GetSkinMats
  (bind _body (CallFunction|GetBodyMeshes))
  (bind _skeletalmesh (Variables|/Script/Engine.SkinnedMeshComponent|GetSkeletalMesh _body))
  (bind _materials (Variables|/Script/Engine.SkeletalMesh|GetMaterials _skeletalmesh))
  (Variables|Default|GetFaceMat
    (:then
      _)
    (:else
      (bind _returnvalue (Rendering|Material|CreateDynamicMaterialInstance (.MaterialInterface (Utilities|Struct|BreakSkeletalMaterial (Utilities|Array|Get(acopy) _materials))) "None" "Transient" :!class /Script/Engine.KismetMaterialLibrary))
      (Variables|Default|SetFaceMat _returnvalue)))
  (Variables|Default|GetTorsoMat
    (:then
      _)
    (:else
      (bind _returnvalue_2 (Rendering|Material|CreateDynamicMaterialInstance (.MaterialInterface (Utilities|Struct|BreakSkeletalMaterial (Utilities|Array|Get(acopy) _materials 3))) "None" "Transient" :!class /Script/Engine.KismetMaterialLibrary))
      (Variables|Default|SetTorsoMat _returnvalue_2)))
  (Variables|Default|GetLegsMat
    (:then
      _)
    (:else
      (bind _returnvalue_3 (Rendering|Material|CreateDynamicMaterialInstance (.MaterialInterface (Utilities|Struct|BreakSkeletalMaterial (Utilities|Array|Get(acopy) _materials 4))) "None" "Transient" :!class /Script/Engine.KismetMaterialLibrary))
      (Variables|Default|SetLegsMat _returnvalue_3)))
  (Variables|Default|GetArmsMat
    (:then
      _)
    (:else
      (bind _returnvalue_4 (Rendering|Material|CreateDynamicMaterialInstance (.MaterialInterface (Utilities|Struct|BreakSkeletalMaterial (Utilities|Array|Get(acopy) _materials 6))) "None" "Transient" :!class /Script/Engine.KismetMaterialLibrary))
      (Variables|Default|SetArmsMat _returnvalue_4)))
  (Variables|Default|GetLipsMat
    (:then
      _)
    (:else
      (bind _returnvalue_5 (Rendering|Material|CreateDynamicMaterialInstance (.MaterialInterface (Utilities|Struct|BreakSkeletalMaterial (Utilities|Array|Get(acopy) _materials 1))) "None" "Transient" :!class /Script/Engine.KismetMaterialLibrary))
      (Variables|Default|SetLipsMat _returnvalue_5)))
  (Variables|Default|GetNailsHandMat
    (:then
      _)
    (:else
      (bind _returnvalue_6 (Rendering|Material|CreateDynamicMaterialInstance (.MaterialInterface (Utilities|Struct|BreakSkeletalMaterial (Utilities|Array|Get(acopy) _materials 9))) "None" "Transient" :!class /Script/Engine.KismetMaterialLibrary))
      (Variables|Default|SetNailsHandMat _returnvalue_6)))
  (Variables|Default|GetNailsFeetMat
    (:then
      _)
    (:else
      (bind _returnvalue_7 (Rendering|Material|CreateDynamicMaterialInstance (.MaterialInterface (Utilities|Struct|BreakSkeletalMaterial (Utilities|Array|Get(acopy) _materials 10))) "None" "Transient" :!class /Script/Engine.KismetMaterialLibrary))
      (Variables|Default|SetNailsFeetMat _returnvalue_7)))
  (return (Variables|Default|GetFaceMat) (Variables|Default|GetTorsoMat) (Variables|Default|GetLegsMat) (Variables|Default|GetArmsMat) (Variables|Default|GetLipsMat) (Variables|Default|GetNailsHandMat) (Variables|Default|GetNailsFeetMat)))

(fn ChangeEyesColor
  (params (Color :type Linear%20Color%20Structure))
  (bind _body (CallFunction|GetBodyMeshes))
  (bind _returnvalue (Rendering|Material|CreateDynamicMaterialInstance _body 7 (Rendering|Material|GetMaterial _body 7) "None" :!class /Script/Engine.PrimitiveComponent))
  (LocalVariables|SetDynMat _returnvalue)
  (Rendering|Material|SetVectorParameterValue (LocalVariables|GetDynMat) "EyeColor" Color :!class /Script/Engine.MaterialInstanceDynamic)
  (Rendering|Material|SetMaterial _body 7 (LocalVariables|GetDynMat))
  (bind _returnvalue_2 (Rendering|Material|CreateDynamicMaterialInstance _body 13 (Rendering|Material|GetMaterial _body 13) "None" :!class /Script/Engine.PrimitiveComponent))
  (LocalVariables|SetDynMat2 _returnvalue_2)
  (Rendering|Material|SetVectorParameterValue (LocalVariables|GetDynMat2) "EyeColor" Color :!class /Script/Engine.MaterialInstanceDynamic)
  (Rendering|Material|SetMaterial _body 13 (LocalVariables|GetDynMat2))
  (return true))

(fn ChangeLipsColor
  (params (Value :type Linear%20Color%20Structure))
  (Rendering|Material|SetVectorParameterValue (Variables|Default|GetLipsMat) "SkinColor" Value :!class /Script/Engine.MaterialInstanceDynamic)
  (return true))

(fn ChangeNailsColor
  (params (Value :type Linear%20Color%20Structure))
  (Rendering|Material|SetVectorParameterValue (Variables|Default|GetNailsHandMat) "Diffuse Color" Value :!class /Script/Engine.MaterialInstanceDynamic)
  (return true))

(fn ApplyNewSkin
  (params (SkinInfoStruct :type Skin%20Info%20Struct%20Structure%20%28by%20ref%29))
  (bind (_name _arms_diffuse _face_diffuse _torso_diffuse _legs_diffuse) (Utilities|Struct|BreakSkinInfoStruct SkinInfoStruct))
  (Rendering|Material|SetTextureParameterValue (Variables|Default|GetFaceMat) "Diffuse Color Texture" _face_diffuse)
  (Rendering|Material|SetTextureParameterValue (Variables|Default|GetTorsoMat) "Diffuse Color Texture" _torso_diffuse)
  (Rendering|Material|SetTextureParameterValue (Variables|Default|GetLegsMat) "Diffuse Color Texture" _legs_diffuse)
  (Rendering|Material|SetTextureParameterValue (Variables|Default|GetArmsMat) "Diffuse Color Texture" _arms_diffuse))

(fn ChangeSkinRoug
  (params (Index :type Integer))
  (Rendering|Material|SetScalarParameterValue (Variables|Default|GetFaceMat) "Roughness Offset" (Utilities|Select :Index Index :Option%200 0.65 :Option%201 0.55 :Option%202 0.45 :Option%203 0.35 :Option%204 0.25 :Option%205 0.15) :!class /Script/Engine.MaterialInstanceDynamic))

(fn ChangeLipsRoug
  (params (Index :type Integer))
  (Rendering|Material|SetScalarParameterValue (Variables|Default|GetLipsMat) "Roughness Offset" (Utilities|Select :Index Index :Option%200 0.65 :Option%201 0.55 :Option%202 0.45 :Option%203 0.35 :Option%204 0.25 :Option%205 0.15) :!class /Script/Engine.MaterialInstanceDynamic))

(fn ChangeNailsRoug
  (params (Index :type Integer))
  (Rendering|Material|SetScalarParameterValue (Variables|Default|GetNailsHandMat) "Roughness" (Utilities|Select :Index Index :Option%200 0.0 :Option%201 0.2 :Option%202 0.3 :Option%203 0.5 :Option%204 0.75 :Option%205 1.0) :!class /Script/Engine.MaterialInstanceDynamic))

(fn ChangeCloth
  (params (Type :type ClothTypesEnum%20Enum :default "NewEnumerator0") (Row :type Name) (SetIndex :type Integer))
  (bind (_body _hair _cloth _shoes _jacket _pants _shirt _underwear) (CallFunction|GetBodyMeshes))
  (bind (_body_2 _hair_2 _cloth_2 _shoes_2 _jacket_2 _pants_2 _shirt_2 _underwear_2) (CallFunction|GetBodyMeshes))
  (bind (_body_3 _hair_3 _cloth_3 _shoes_3 _jacket_3 _pants_3 _shirt_3 _underwear_3) (CallFunction|GetBodyMeshes))
  (bind _returnvalue (Utilities|Select :Index Type :NewEnumerator0 _shoes_2 :NewEnumerator1 _cloth_2 :NewEnumerator2 _pants_2 :NewEnumerator3 _jacket_2 :NewEnumerator4 0 :NewEnumerator5 _shirt_2 :NewEnumerator6 0 :NewEnumerator7 0 :NewEnumerator8 _underwear_2))
  (if (Utilities|Name|NotEqual(Name) Row "None")
    (bind _returnvalue_2 (Utilities|GetDataTableRow "/Game/ProceduralGeneration/DT_Cloth.DT_Cloth" Row)
      (:then
        (Class|SkinnedMeshComponent|SetSkeletalMesh _returnvalue (.Mesh (Utilities|Struct|BreakClothStruct _returnvalue_2)) false)
        (CallFunction|ChangeClothMaterial _returnvalue (Utilities|Array|Get(acopy) (.Materials (Utilities|Struct|BreakClothStruct _returnvalue_2)) SetIndex) _returnvalue_2)
        (if true
          (switch Utilities|FlowControl|Switch|SwitchonClothTypesEnum Type
            (:NewEnumerator0
              _)
            (:NewEnumerator1
              (Class|SkinnedMeshComponent|SetSkeletalMesh _pants_3 0 true)
              (Class|SkinnedMeshComponent|SetSkeletalMesh _shirt_3 0 true)
              (Class|SkinnedMeshComponent|SetSkeletalMesh _underwear_3 0 true)
              (return true))
            (:NewEnumerator2
              (Class|SkinnedMeshComponent|SetSkeletalMesh _cloth_3 0 true)
              (Class|SkinnedMeshComponent|SetSkeletalMesh _underwear_3 0 true)
              (return true))
            (:NewEnumerator3
              _)
            (:NewEnumerator5
              (Class|SkinnedMeshComponent|SetSkeletalMesh _cloth_3 0 true)
              (Class|SkinnedMeshComponent|SetSkeletalMesh _underwear_3 0 true)
              (return true))
            (:NewEnumerator8
              (Class|SkinnedMeshComponent|SetSkeletalMesh _cloth_3 0 true)
              (Class|SkinnedMeshComponent|SetSkeletalMesh _pants_3 0 true)
              (Class|SkinnedMeshComponent|SetSkeletalMesh _shirt_3 0 true)
              (return true)))
          (return true)
          (else
            (switch Utilities|FlowControl|Switch|SwitchonClothTypesEnum Type
              (:NewEnumerator0
                _)
              (:NewEnumerator1
                (Class|SkinnedMeshComponent|SetSkeletalMesh _cloth 0 true))
              (:NewEnumerator2
                (Class|SkinnedMeshComponent|SetSkeletalMesh _pants 0 true))
              (:NewEnumerator3
                (Class|SkinnedMeshComponent|SetSkeletalMesh _jacket 0 true))
              (:NewEnumerator5
                (Class|SkinnedMeshComponent|SetSkeletalMesh _shirt 0 true))
              (:NewEnumerator8
                (Class|SkinnedMeshComponent|SetSkeletalMesh _underwear 0 true)))
            (return true))))
      (:RowNotFound
        (return false)))
    (else
      (Class|SkinnedMeshComponent|SetSkeletalMesh _returnvalue 0 false))))

(fn ChangeClothMaterial
  (params (Component :type Primitive%20Component%20Object%20Reference) (Material :type Multiple%20Materials%20Struct%20Structure%20%28by%20ref%29) (Cloth :type Cloth%20Struct%20Structure%20%28by%20ref%29))
  (for (_array_element _array_index) (.Materials (Utilities|Struct|BreakMultipleMaterialsStruct Material))
    (Rendering|Material|SetMaterial Component _array_index _array_element))
  (return true))

(fn ChangeClothColor
  (params (Color :type Linear%20Color%20Structure) (Type :type ClothTypesEnum%20Enum :default "NewEnumerator0") (Index :type Integer))
  (bind (_body _hair _cloth _shoes _jacket _pants _shirt _underwear) (CallFunction|GetBodyMeshes))
  (bind _returnvalue (Utilities|Select :Index Type :NewEnumerator0 _shoes :NewEnumerator1 _cloth :NewEnumerator2 _pants :NewEnumerator3 _jacket :NewEnumerator4 0 :NewEnumerator5 _shirt :NewEnumerator6 0 :NewEnumerator7 0 :NewEnumerator8 _underwear))
  (Utilities|IsValid _returnvalue
    (:Is%20Valid
      (Rendering|Material|SetVectorParameterValueonMaterials _returnvalue (Utilities|Select :Index Index :Option%200 "Color" :Option%201 "Color2" :Option%202 "Color3") (Math|Conversions|ToVector(LinearColor) Color))
      (bind _aspc_character_creator (Utilities|Casting|CastToPC_CharacterCreator (Game|GetPlayerController 0)))
      (switch int Index
        (:0
          (bind _structout (Utilities|Struct|SetmembersinCCEquipsStruct (Default|GetEquipbyType _aspc_character_creator Type) Color))
          (Default|SetEquipbyType _aspc_character_creator Type _structout))
        (:1
          (bind _structout_2 (Utilities|Struct|SetmembersinCCEquipsStruct (Default|GetEquipbyType _aspc_character_creator Type) Color))
          (Default|SetEquipbyType _aspc_character_creator Type _structout_2))
        (:2
          (bind _structout_3 (Utilities|Struct|SetmembersinCCEquipsStruct (Default|GetEquipbyType _aspc_character_creator Type) Color))
          (Default|SetEquipbyType _aspc_character_creator Type _structout_3)))
      (return true))))