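; Player controller for the scene creator: shows its UI and applies saved characters to the selected scene actor.
; Loading restores body shape keys, hair, makeup, skin, colors and roughness; other clothing restore logic is unconnected.
; Scene selection refreshes animation slots in right-box widgets, and animation choices propagate to the scene's BP_SceneActor children.
; It also holds play, pause and rate state, and a left click off the active character deselects it.
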(event Custom|SelectScene
  (params (Scene :type BP%20Scene%20Base%20Object%20Reference))
  (Variables|Default|SetSceneSelected Scene)
  (bind _foundwidgets (Widget|GetAllWidgetsOfClass "/Game/SceneCreator/WBP_SC_RightBox.WBP_SC_RightBox_C" false))
  (for _array_element _foundwidgets
    (Default|SpawnAnimationSlots _array_element (Variables|Default|GetSceneSelected))))

(event Custom|SelectAnimation
  (params (ID :type Integer))
  (bind _sceneselected (Variables|Default|GetSceneSelected))
  (bind _keys (Utilities|Map|Keys (Variables|/Game/SceneCreator/BP_SceneBase.BP_SceneBase_C|GetAnims _sceneselected)))
  (Variables|Default|SetSelectedAnim (Utilities|Array|Get(acopy) _keys ID))
  (for _array_element (Actor|GetAllChildActors _sceneselected true)
    (bind _asbp_scene_actor (Utilities|Casting|CastToBP_SceneActor _array_element))
    (Default|SelectAnimation _asbp_scene_actor ID)))

(event Custom|PlayAnim
  (params (PlayAnim? :type Boolean))
  (Variables|Default|SetPlayAnim? PlayAnim?)
  (Variables|Default|SetPaused? false)
  (Variables|Default|SetPlayRate 1.0))

(event Custom|ChangePlayRate
  (params (PlayRate :type Float%20%28single-precision%29))
  (Variables|Default|SetPlayRate PlayRate))

(event Custom|PauseAnim
  (bind _output_get (Variables|Default|SetPaused? (not (Variables|Default|GetPaused?))))
  (if _output_get
    (Variables|Default|SetPlayRate 0.0)
    (else
      (Variables|Default|SetPlayRate 1.0))))

(event Custom|LoadSavedCharacter
  (params (SavedCharacter :type Save%20Character%20Struct%20Structure))
  (bind (_female _name _body _bodyshapes _equips _bodycolor _eyescolor _lipscolor _nailscolor _savedate _skininfo _skinroug _lipsroug _nailsroug) (Utilities|Struct|BreakSaveCharacterStruct SavedCharacter))
  (bind _actor_to_load (Variables|Default|GetActor%20to%20Load))
  (bind _actor_to_load_2 (Variables|Default|GetActor%20to%20Load))
  (bind _actor_to_load_3 (Variables|Default|GetActor%20to%20Load))
  (Utilities|Map|Clear (Variables|Default|GetSavedMeshes))
  (Utilities|Platform|CollectGarbage)
  (Variables|Default|GetActor%20to%20Load
    (:then
      (Utilities|FlowControl|Sequence
        (:then_0
          (CallFunction|LoadSavedShapes _bodyshapes _actor_to_load))
        (:then_1
          (CallFunction|LoadSavedEquips _equips _actor_to_load))
        (:then_2
          (Default|ChangeSkinColor _actor_to_load_3 _bodycolor)
          (Default|ChangeEyesColor _actor_to_load_3 _eyescolor)
          (Default|ChangeLipsColor _actor_to_load_3 _lipscolor)
          (Default|ChangeNailsColor _actor_to_load_3 _nailscolor))
        (:then_3
          (Default|ApplyNewSkin _actor_to_load_3 _skininfo))
        (:then_4
          (Default|ChangeSkinRoug _actor_to_load_2 _skinroug)
          (Default|ChangeLipsRoug _actor_to_load_2 _lipsroug)
          (Default|ChangeNailsRoug _actor_to_load_2 _nailsroug))))
    (:else
      (Development|PrintString "Select Character" true true "(R=1.000000,G=0.000000,B=0.000000,A=1.000000)" 5.0))))

(event EventBeginPlay
  (bind _returnvalue (UserInterface|CreateWidget "/Game/SceneCreator/WBP_SceneCreator.WBP_SceneCreator_C"))
  (UserInterface|Viewport|AddtoViewport _returnvalue 0))

(event Input|MouseEvents|LeftMouseButton
  (params (Key :type Key%20Structure :default "None"))
  (:Pressed
    (Utilities|IsValid (Variables|Default|GetActor%20to%20Load)
      (:Is%20Valid
        (if (!= (.HitActor (Collision|BreakHitResult (.HitResult (Game|Player|GetHitResultUnderCursorbyChannel "TraceTypeQuery1" true)))) (Variables|/Script/Engine.ChildActorComponent|GetChildActor (Variables|/Game/SceneCreator/BP_SceneActor.BP_SceneActor_C|GetChildActor_Character (Variables|Default|GetActor%20to%20Load))))
          (bind _actor_to_load (Variables|Default|GetActor%20to%20Load)
            (:then
              (bind _asbp_cc_character_viewer (Utilities|Casting|CastToBP_CC_CharacterViewer (Variables|/Script/Engine.ChildActorComponent|GetChildActor (Variables|/Game/SceneCreator/BP_SceneActor.BP_SceneActor_C|GetChildActor_Character _actor_to_load))))
              (Default|MouseOff _actor_to_load (Variables|/Script/Engine.Character|GetMesh _asbp_cc_character_viewer))
              (Variables|Default|SetActor%20to%20Load 0))
            (:else)))))))

(fn ConstructionScript)

(fn GetCC
  (return 0))

(fn LoadSavedShapes
  (params (Shapes :type Map%20of%20Strings%20to%20Float%20%28single-precision%29s) (SceneActor :type BP%20Scene%20Actor%20Object%20Reference))
  (bind _asbp_cc_character_viewer (Utilities|Casting|CastToBP_CC_CharacterViewer (Variables|/Script/Engine.ChildActorComponent|GetChildActor (Variables|/Game/SceneCreator/BP_SceneActor.BP_SceneActor_C|GetChildActor_Character SceneActor)))
    (:then
      (CallFunction|ApplyShapeKeys (Variables|/Script/Engine.Character|GetMesh _asbp_cc_character_viewer) Shapes)
      (return true))
    (:CastFailed
      (return false))))

(fn LoadSavedEquips
  (params (Equips :type Array%20of%20CC%20Equips%20Struct%20Structures) (SCactor :type BP%20Scene%20Actor%20Object%20Reference))
  (for _array_element Equips
    (switch Utilities|FlowControl|Switch|SwitchonClothTypesEnum (.Type (Utilities|Struct|BreakCCEquipsStruct _array_element))
      (:NewEnumerator4
        (Default|ChangeHair SCactor (.Mesh (Utilities|Struct|BreakCCEquipsStruct _array_element)))
        (Utilities|FlowControl|Sequence
          (:then_0
            (Default|ChangeHairColor SCactor (.Color (Utilities|Struct|BreakCCEquipsStruct _array_element))))
          (:then_1
            (Default|ChangeHairColor SCactor (.Color2 (Utilities|Struct|BreakCCEquipsStruct _array_element)) 1))))
      (:NewEnumerator6
        (Default|ChangeMakeUp SCactor (.Makeup (Utilities|Struct|BreakCCEquipsStruct _array_element)) "eyes")
        (Default|ChangeMakeUpColor SCactor (.Color (Utilities|Struct|BreakCCEquipsStruct _array_element)) "eyes"))
      (:NewEnumerator7
        (Default|ChangeMakeUp SCactor (.Makeup (Utilities|Struct|BreakCCEquipsStruct _array_element)) "face")
        (Default|ChangeMakeUpColor SCactor (.Color (Utilities|Struct|BreakCCEquipsStruct _array_element)) "face"))))
  (return true))